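; Flying enemy that homes in on the player, takes bullet damage and backs off after contact.
; Each tick it queries AI Perception for the player pawn and, if the first stimulus was sensed, calls FlyAtPlayer with the player's camera location.
; Capsule overlaps call ReduceHealth for bullets, or RetreatFunc away from the player to avoid rapid repeat overlaps.
; Movement and health logic live outside these graphs.
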(event `self.ReceiveTick`
  (params (DeltaSeconds :type "Float (single-precision)"))
  (`parent.ReceiveTick` DeltaSeconds)
  ;[1 1 1] triggers move to player function when this enemy can see the player pawn
  (bind _info (`AIPerceptionComponent.GetActorsPerception` (`self.AIPerception`) (`GameplayStatics.GetPlayerPawn` 0)))
  (bind (_target _lastsensedstimuli) (break `ActorPerceptionBlueprintInfo` _info))
  (if (> (`KismetArrayLibrary.Array_Length` _lastsensedstimuli) 0)
    (if (`.bSuccessfullySensed` (break `AIStimulus` (`|GetArrayItem` _lastsensedstimuli)))
      (`self.flyAtPlayer` (`SceneComponent.K2_GetComponentLocation` (`self.GetComponentByClass` _target "/Script/Engine.CameraComponent"))))))

(event `self.Capsule.OnComponentBeginOverlap`
  (params (OverlappedComponent :type "PrimitiveComponent Object Reference") (OtherActor :type "Actor Object Reference") (OtherComp :type "PrimitiveComponent Object Reference") (OtherBodyIndex :type Integer) (bFromSweep :type Boolean) (SweepResult :type "HitResult Structure (by ref)"))
  (bind _returnvalue (`self.K2_GetActorLocation`))
  (bind _returnvalue_2 (`ActorComponent.GetOwner` OtherComp))
  (bind _returnvalue_3 (`GameplayStatics.GetObjectClass` _returnvalue_2))
  ;[1 1 1] detect if enemy is overlapping with a capsule component
  (if (`KismetMathLibrary.ClassIsChildOf` (`GameplayStatics.GetObjectClass` OtherComp) "/Script/Engine.CapsuleComponent")
    ;[1 1 1] if owner of capsul component is a bullet reduce this enemy's health
    (if (`KismetMathLibrary.ClassIsChildOf` _returnvalue_3 "/Script/UE5_AR.Bullet")
      (`self.ReduceHealth`)
      (else
        ;[1 1 1] if the capsule component belongs to the player, retreat 300 units in the opposite direction. This is done so the player doesn't repeatedly overlap with the same enemy in a short burst
        (if (`KismetMathLibrary.ClassIsChildOf` _returnvalue_3 "/Game/Blueprints/newPlayerPawn.newPlayerPawn_C")
          (`self.RetreatFunc` (+ (* (`KismetMathLibrary.GetDirectionUnitVector` (`self.K2_GetActorLocation` _returnvalue_2) _returnvalue) (300.0 300.0 300.0)) _returnvalue)))))))

(fn `UserConstructionScript`
  (`parent.UserConstructionScript`))