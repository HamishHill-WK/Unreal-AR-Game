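; Enemy Blueprint with health, an EnemyUI widget component and death handling.
; On begin play it passes itself to the widget, then each tick pushes the bar visibility flag and triggers delayed death once health is depleted.
; The smashHit event applies repeated damage to a living enemy, with a shorter death delay if it kills.
; Damage and Dead are thin wrappers around MDamage and MDead.
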(event `ReceiveBeginPlay_1`
  (bind _asenemy_ui (cast `` (`WidgetComponent.GetUserWidgetObject` (`self.enemyUI`))))
  (set `/Game/Blueprints/enemy302.enemyBP` self _asenemy_ui))

(event `ReceiveTick_1`
  (params (DeltaSeconds :type "Float (single-precision)"))
  (bind _asenemy_ui (cast `` (`WidgetComponent.GetUserWidgetObject` (`self.enemyUI`))))
  (set `/Game/Blueprints/enemy302.visible` (`self.b_barVisible`) _asenemy_ui)
  (if (<= (`self.fl_enemyHealth`) 0.0)
    (`KismetSystemLibrary.Delay` 0.5)
    (`self.dead`)))

(event `smashHit`
  (bind _fl_enemyhealth (`self.fl_enemyHealth`))
  (if (not (<= _fl_enemyhealth 0.0))
    (for _ (range 7)
      (`self.damage`))
    (if (<= _fl_enemyhealth 0.0)
      (`KismetSystemLibrary.Delay` 0.05)
      (`self.dead`))))

(fn `damage`
  (`self.m_damage`))

(fn `dead`
  (`self.m_dead`))

(fn `UserConstructionScript`)