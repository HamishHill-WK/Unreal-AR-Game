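; newPlayerPawn is the player pawn Blueprint built on C++ CustomARPawn, handling the player's HUD, sounds and damage from enemies.
; BeginPlay creates the UI_BP widget and shows the start button.
; Events declared in C++ toggle the crosshair, health and ammo widgets, start music once, play laser shots and show the death screen.
; Capsule overlaps with an Enemy-owned capsule component call ReduceHealth.
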(event `self.ReceiveBeginPlay`
  (bind _playerui (`self.PlayerUI`))
  ;[1 1 1] adds ui to player view
  (`AudioComponent.Stop` (`self.Audio`))
  (bind _returnvalue (`|CreateWidget` "/Game/Blueprints/UI_BP.UI_BP_C"))
  (bind _output_get (set `self.PlayerUI` _returnvalue))
  (`UserWidget.AddToViewport` _output_get 0)
  (`/Game/Blueprints/UI_BP.SetWidgetVisibility` _playerui true (`/Game/Blueprints/UI_BP.StartGameButton` _playerui)))

(event `self.UISetCrossHair`
  (params (showCH :type Boolean))
  (bind _playerui (`self.PlayerUI`))
  ;[1 1 1] These functions are declared in CustomARPawn.h but defined here. The events can be called from script or blueprints
  (`/Game/Blueprints/UI_BP.SetWidgetVisibility` _playerui showCH (`/Game/Blueprints/UI_BP.CrosshairImg` _playerui))
  (`/Game/Blueprints/UI_BP.SetWidgetVisibility` _playerui showCH (`/Game/Blueprints/UI_BP.HealthBar` _playerui))
  (`/Game/Blueprints/UI_BP.SetWidgetVisibility` _playerui showCH (`/Game/Blueprints/UI_BP.AmmoCounter` _playerui))
  (if showCH
    (`/Engine/EditorBlueprintResources/StandardMacros.DoOnce` false
      (:`Completed`
        (`GameplayStatics.PlaySound2D` "/Game/Assets/Audio/MainSong1__Cue.MainSong1__Cue" 1.0 1.0 0.0 null null)))))

(event `self.UISetStartButton`
  (params (showSB :type Boolean))
  (bind _playerui (`self.PlayerUI`))
  ;[1 1 1] These functions are declared in CustomARPawn.h but defined here. The events can be called from script or blueprints
  (`/Game/Blueprints/UI_BP.SetWidgetVisibility` _playerui showSB (`/Game/Blueprints/UI_BP.StartGameButton` _playerui)))

(event `self.playerDead`
  ;[1 1 1] These functions are declared in CustomARPawn.h but defined here. The events can be called from script or blueprints
  (`self.PlayerDeathScreen` "You Died"))

(event `self.ShootSound`
  ;[1 1 1] These functions are declared in CustomARPawn.h but defined here. The events can be called from script or blueprints
  (`GameplayStatics.PlaySound2D` "/Game/Assets/Audio/Laser1_Cue.Laser1_Cue" 1.0 1.0 0.0 null null))

(event `self.Capsule.OnComponentBeginOverlap`
  (params (OverlappedComponent :type "PrimitiveComponent Object Reference") (OtherActor :type "Actor Object Reference") (OtherComp :type "PrimitiveComponent Object Reference") (OtherBodyIndex :type Integer) (bFromSweep :type Boolean) (SweepResult :type "HitResult Structure (by ref)"))
  ;[1 1 1] reduce health when overlapping enemy obejct
  (if (`KismetMathLibrary.ClassIsChildOf` (`GameplayStatics.GetObjectClass` OtherComp) "/Script/Engine.CapsuleComponent")
    (if (`KismetMathLibrary.ClassIsChildOf` (`GameplayStatics.GetObjectClass` (`ActorComponent.GetOwner` OtherComp)) "/Game/Blueprints/Enemy.Enemy_C")
      (`self.ReduceHealth`))))

(fn `PlayerDeathScreen`
  (params (EndText :type Text))
  (bind _playerui (`self.PlayerUI`))
  (`/Game/Blueprints/UI_BP.SetWidgetVisibility` _playerui false (`/Game/Blueprints/UI_BP.OpenMenu` _playerui))
  (set `/Game/Blueprints/UI_BP.EndScreenText` EndText _playerui)
  (`/Game/Blueprints/UI_BP.SetWidgetVisibility` _playerui true (`/Game/Blueprints/UI_BP.EndScreen` _playerui)))

(fn `UserConstructionScript`)